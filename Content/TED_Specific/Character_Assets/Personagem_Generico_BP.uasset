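; Generic player character Blueprint with movement, spring-arm camera, double jump, two-button combo attacks and health.
; Velocity decides whether side input strafes or turns and whether camera yaw also rotates the character; camera pitch is clamped.
; Attack inputs branch on the previous attack to play combo montages, gated by playback position.
; Lethal damage from a player-controller instigator triggers authority-only death, which unpossesses and destroys the actor for respawn.
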(event `self.ReceiveTick`
  (params (DeltaSeconds :type "Float (single-precision)")))

(event `self.ReceiveBeginPlay`)

(event `self.ReceiveAnyDamage`
  (params (Damage :type "Float (single-precision)") (DamageType :type "DamageType Object Reference") (InstigatedBy :type "Controller Object Reference") (DamageCauser :type "Actor Object Reference"))
  (bind _returnvalue (- (`self.CurHealth`) (`KismetMathLibrary.FFloor` Damage)))
  ;[1 0.1638 0.124] Aplica dano ao personagem de fato
  (if (<= _returnvalue 0)
    (set `self.CurHealth` 0)
    (bind _asplayer_controller_bp (cast `/Game/TED_Specific/Character_Assets/Player_Controller_BP` InstigatedBy))
    (`self.DeathEvent` _asplayer_controller_bp)
    (else
      (set `self.CurHealth` _returnvalue))))

(event `DeathEvent`
  (params (WhoKilled :type "/Game/TED_Specific/Character_Assets/Player_Controller_BP Object Reference"))
  ;[1 0.1638 0.124] Executa a morte do personagem, independente do motivo
  (`/Engine/EditorBlueprintResources/ActorMacros.Switch Has Authority`
    (:`Authority`
      (bind _is_dead (`self.Death_Confirmation`))
      (if _is_dead
        (`self.Server_DeathNotify`)
        (`self.K2_DestroyActor`) ; A destruíção do ator ativa a notificação do controlador para permitir o respawn
      ))
    (:`Remote`
      (`KismetSystemLibrary.PrintString` "OnlyServerMayKill"))))

(event `Server_DeathNotify`
  ;[1 1 1] Notifica o servidor da morte
)

(event `InputAxis|RunForward`
  (params (AxisValue :type "Float (single-precision)"))
  ;[0.2531 0.3765 1] Funções de movimento
  (`self.Run_FWD/BWD` AxisValue))

(event `InputAction|Atk_1_Inp`
  (params (Key :type "Key Structure"))
  ;[0.08351 1 0.1068] Funções de Ataque
  (:`Pressed`
    (bind _isending (`self.Test_MontageEnded`)
      (:`Playing`
        (if _isending
          (switch `int` (`self.WhatPreviousAtk`) :!label _label
            (:`0`
              (`self.Atk1_Call`))
            (:`1`
              (`self.Atk1_1_Call`))
            (:`2`
              (`self.Atk2_1_Call`)))
          (else
            (`KismetSystemLibrary.PrintString` "Animação não acabou"))))
      (:`NotPlaying`
        (goto _label)))))

(event `InputAxis|PanHor`
  (params (AxisValue :type "Float (single-precision)"))
  ;[0.2531 0.3765 1] Funções de movimento
  (`self.CamRotation_X` AxisValue))

(event `Atk1_Visual`
  ;[0.08351 1 0.1068] Funções de Ataque
  (`self.PlayAnimMontage` "/Game/TED_Specific/Character_Assets/Proxy_Ted/Mont_Combo_1.Mont_Combo_1"))

(event `Atk1_1_Visual`
  ;[0.08351 1 0.1068] Funções de Ataque
  (`self.PlayAnimMontage` "/Game/TED_Specific/Character_Assets/Proxy_Ted/Mont_Combo_1_1.Mont_Combo_1_1"))

(event `Atk2_1_Visual`
  ;[0.08351 1 0.1068] Funções de Ataque
  (`self.PlayAnimMontage` "/Game/TED_Specific/Character_Assets/Proxy_Ted/Mont_Combo_2_1.Mont_Combo_2_1"))

(event `Atk1_Call`
  ;[0.08351 1 0.1068] Funções de Ataque
  (set `self.WhatPreviousAtk` 1)
  (`self.Atk1_Visual`)
  (`self.Atk1_Mech`))

(event `Atk1_1_Call`
  ;[0.08351 1 0.1068] Funções de Ataque
  (set `self.WhatPreviousAtk` 0)
  (`self.Atk1_1_Visual`))

(event `Atk2_1_Call`
  ;[0.08351 1 0.1068] Funções de Ataque
  (set `self.WhatPreviousAtk` 0)
  (`self.Atk2_1_Visual`))

(event `Atk1_Mech`
  ;[0.08351 1 0.1068] Funções de Ataque
)

(event `Atk2_Visual`
  ;[0.08351 1 0.1068] Funções de Ataque
  (`self.PlayAnimMontage` "/Game/TED_Specific/Character_Assets/Proxy_Ted/Mont_Combo_2.Mont_Combo_2"))

(event `Atk1_2_Visual`
  ;[0.08351 1 0.1068] Funções de Ataque
  (`self.PlayAnimMontage` "/Game/TED_Specific/Character_Assets/Proxy_Ted/Mont_Combo_1_2.Mont_Combo_1_2"))

(event `Atk2_2_Visual`
  ;[0.08351 1 0.1068] Funções de Ataque
  (`self.PlayAnimMontage` "/Game/TED_Specific/Character_Assets/Proxy_Ted/Mont_Combo_2_2.Mont_Combo_2_2"))

(event `Atk2_Call`
  ;[0.08351 1 0.1068] Funções de Ataque
  (set `self.WhatPreviousAtk` 2)
  (`self.Atk2_Visual`))

(event `Atk1_2_Call`
  ;[0.08351 1 0.1068] Funções de Ataque
  (set `self.WhatPreviousAtk` 0)
  (`self.Atk1_2_Visual`))

(event `Atk2_2_Call`
  ;[0.08351 1 0.1068] Funções de Ataque
  (set `self.WhatPreviousAtk` 0)
  (`self.Atk2_2_Visual`))

(event `InputAxis|PanVert`
  (params (AxisValue :type "Float (single-precision)"))
  ;[0.2531 0.3765 1] Funções de movimento
  (`self.CamRotation_Y` AxisValue))

(event `InputAxis|MoveTurnSide`
  (params (AxisValue :type "Float (single-precision)"))
  ;[0.2531 0.3765 1] Funções de movimento
  (`self.Sideways_Move/Turn` AxisValue))

(event `InputAction|Atk_2_Inp`
  (params (Key :type "Key Structure"))
  ;[0.08351 1 0.1068] Funções de Ataque
  (:`Pressed`
    (bind _isending (`self.Test_MontageEnded`)
      (:`Playing`
        (if _isending
          (switch `int` (`self.WhatPreviousAtk`) :!label _label_2
            (:`0`
              (`self.Atk2_Call`))
            (:`1`
              (`self.Atk2_1_Call`))
            (:`2`
              (`self.Atk2_2_Call`)))
          (else
            (`KismetSystemLibrary.PrintString` "Animação não acabou"))))
      (:`NotPlaying`
        (goto _label_2)))))

(event `InputAction|Jump_Inp`
  (params (Key :type "Key Structure"))
  ;[0.2531 0.3765 1] Funções de movimento
  (:`Pressed`
    (`self.DoubleJump`)))

(event `self.OnLanded`
  (params (Hit :type "HitResult Structure (by ref)"))
  ;[0.2531 0.3765 1] Funções de movimento
  (set `self.JumpNum` 0))

(fn `BlockCall`)

(fn `CamRotation_X`
  (params (NewParam :type "Float (double-precision)"))
  ;[0.2531 0.3765 1] Rotação da camera na horizontal
  ;;[1 1 1] Adiciona rotação somente na câmera se o personagem estiver parado e retorna.
  (`SceneComponent.K2_AddRelativeRotation` (`self.SpringArm`) (`KismetMathLibrary.MakeRotator` 0.0 0.0 NewParam) false false)
  (if (`self.Test_Velocity`)
    ;;[0.2531 0.3765 1] Adiciona rotação também sobre o personagem se ele estiver em movimento.
    (`self.AddControllerYawInput` (* NewParam 0.4))
    (return)
    (else
      (return))))

(fn `CamRotation_Y`
  (params (InputAxis :type "Float (double-precision)"))
  (bind (_toohigh _toolow) (`self.Test_Camera_Rot`))
  (bind _springarm (`self.SpringArm`))
  (bind _springarm_2 (`self.SpringArm`))
  (bind (_relativerotation_roll _relativerotation_pitch _relativerotation_yaw) (`KismetMathLibrary.BreakRotator` (`SceneComponent.RelativeRotation` _springarm_2)))
  (bind (_relativerotation_roll_2 _relativerotation_pitch_2 _relativerotation_yaw_2) (`KismetMathLibrary.BreakRotator` (`SceneComponent.RelativeRotation` _springarm)))
  ;[0.2531 0.3765 1] Rotação da câmera na vertical
  (if _toohigh
    ;;[1 1 1] Trava a rotação da câmera se a rotação dela em "y" for maior que -50º
    (`SceneComponent.K2_SetRelativeRotation` _springarm (`KismetMathLibrary.MakeRotator` _relativerotation_roll_2 -47.99 _relativerotation_yaw_2) false false)
    (elif _toolow
      ;;[1 1 1] Trava a rotação da câmera se a rotação dela em "y" for menor que -50º
      (`SceneComponent.K2_SetRelativeRotation` _springarm_2 (`KismetMathLibrary.MakeRotator` _relativerotation_roll 47.99 _relativerotation_yaw) false false)
      (else
        ;;[1 1 1] Adiciona rotação em "y" se o valor for válido.
        (`SceneComponent.K2_AddRelativeRotation` (`self.SpringArm`) (`KismetMathLibrary.MakeRotator` 0.0 InputAxis) false false))))
  (return))

(fn `CanJumpInternal`
  (returns (ReturnValue :type Boolean))
  (bind _returnvalue (`parent.CanJumpInternal`))
  (return (or _returnvalue (`NavMovementComponent.IsFalling` (`self.CharacterMovement`)))))

(fn `Death_Confirmation`
  (returns (Is_Dead :type Boolean))
  ;[1 0.1638 0.124] Como deve agir ao morrer
  (`/Engine/EditorBlueprintResources/ActorMacros.Switch Has Authority`
    (:`Authority`
      (`self.Test_Is_Dead` ; Teste de redundância, garante que o personagem está morto.
        (:`Is_Dead`
          ;;[1 1 1] Retira a posse do controlador sobre o personagem se ele estiver morto.
          (`KismetSystemLibrary.PrintString` "Morri")
          (bind _asplayer_controller_bp (cast `/Game/TED_Specific/Character_Assets/Player_Controller_BP` (`self.GetController`))
            (:`then`
              (`Controller.UnPossess` _asplayer_controller_bp))
            (:`CastFailed`
              (`KismetSystemLibrary.PrintString` "Death Cast fail" true true (struct :`R` 1.0 :`G` 0.742836 :`B` 0.027617 :`A` 1.0) 20.0)))
          (return true) ; Retorna com um aviso de que o personagem está morto para continuar o processo de morte
        )
        (:`Is_Alive`
          _)))
    (:`Remote`
      _))
  (return false))

(fn `DoubleJump`
  (if (< (`self.JumpNum`) 2)
    (`self.Jump`)
    (`/Engine/EditorBlueprintResources/StandardMacros.IncrementInt` (`self.JumpNum`)
      (:`  `
        (return)))))

(fn `HasKilled`)

(fn `OnRep_Health_De-Buff`)

(fn `ResetComboFN`
  (`KismetSystemLibrary.PrintString` "ResettingCombo" true true (struct :`G` 0.66 :`B` 1.0 :`A` 1.0) 10.0)
  (set `self.IsNewCombo` true)
  (set `self.ComboNumb` 0))

(fn `RiposteCall`)

(fn `Run_FWD/BWD`
  (params (A :type "Float (double-precision)"))
  ;[0.2531 0.3765 1] Função de movimentação frente/costas
  (if (not (`self.IsIncapacitated`))
    (`self.AddMovementInput` (`KismetMathLibrary.GetForwardVector` (`KismetMathLibrary.MakeRotator` 0.0 0.0 (.yaw (`Controller.GetControlRotation` (`GameplayStatics.GetPlayerController` 0))))) (* A 1.0) true)))

(fn `Sideways_Move/Turn`
  (params (NewParam :type "Float (double-precision)"))
  ;[0.2531 0.3765 1] Move ou gira o personagem lateralmente
  (if (`self.Test_Velocity`)
    ;;[1 1 1] Caso o personagem esteja já em movimento é adicionado
    ;; movimento lateral.
    (`self.AddMovementInput` (`KismetMathLibrary.GetRightVector` (`KismetMathLibrary.MakeRotator` 0.0 0.0 (.yaw (`Controller.GetControlRotation` (`GameplayStatics.GetPlayerController` 0))))) NewParam)
    (else
      ;;[1 1 1] Caso o personagem esteja parado ele apenas rotaciona no lugar
      (`self.AddControllerYawInput` NewParam)))
  (return))

(fn `StringTest`
  (for _array_element _
    (`KismetSystemLibrary.PrintString` _array_element true true (struct :`G` 0.66 :`B` 1.0 :`A` 1.0) 5.0)))

(fn `UserConstructionScript`)