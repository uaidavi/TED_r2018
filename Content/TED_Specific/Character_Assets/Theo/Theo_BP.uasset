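; Theo character Blueprint that sets health to 100 and implements a first attack that knocks a character away.
; Atk1Mech takes the first player controller's TargetChar and impulses its movement along the launcher's forward vector, using an authority switch that routes remote calls through LaunchTargetChar.
; The attack collider maintains a possible-target list, but the returned target ignores both that list and the overlap check.
; ApplyLaunch and the damage step are left unreached.
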(event `self.Atk1_Mech`
  (bind _charatked (`self.GetCharToATK`))
  (`/Engine/EditorBlueprintResources/ActorMacros.Switch Has Authority` :!label _label
    (:`Authority`
      (`/Engine/EditorBlueprintResources/StandardMacros.IsValid` (stale `LaunchTargetChar` LaunchingCharacter)
        (:`Is Valid`
          (set `self.DistanceToLaunch` (`self.GetActorForwardVector` (stale `LaunchTargetChar` LaunchingCharacter))))
        (:`Is Not Valid`
          (set `self.DistanceToLaunch` (`self.GetActorForwardVector`)))))
    (:`Remote`
      (`self.LaunchTargetChar` self _charatked)))
  (`CharacterMovementComponent.AddImpulse` (`Character.CharacterMovement` (stale `LaunchTargetChar` LaunchedCharacter)) (* (`self.DistanceToLaunch`) 1800.0) true)
  (`CharacterMovementComponent.AddImpulse` (`Character.CharacterMovement` _charatked) (* (`self.DistanceToLaunch`) 1800.0) true))

(event `LaunchTargetChar`
  (params (LaunchingCharacter :type "/Game/TED_Specific/Character_Assets/Personagem_Generico_BP Object Reference") (LaunchedCharacter :type "/Game/TED_Specific/Character_Assets/Personagem_Generico_BP Object Reference"))
  (goto _label))

(event `self.Atk1_Collider.OnComponentBeginOverlap`
  (params (OverlappedComponent :type "PrimitiveComponent Object Reference") (OtherActor :type "Actor Object Reference") (OtherComp :type "PrimitiveComponent Object Reference") (OtherBodyIndex :type Integer) (bFromSweep :type Boolean) (SweepResult :type "HitResult Structure (by ref)"))
  (bind _aspersonagem_generico_bp (cast `/Game/TED_Specific/Character_Assets/Personagem_Generico_BP` OtherActor))
  (`KismetArrayLibrary.Array_Add` (`self.Atk1PossibleTargets`) _aspersonagem_generico_bp))

(event `self.Atk1_Collider.OnComponentEndOverlap`
  (params (OverlappedComponent :type "PrimitiveComponent Object Reference") (OtherActor :type "Actor Object Reference") (OtherComp :type "PrimitiveComponent Object Reference") (OtherBodyIndex :type Integer))
  (for (_array_element _array_index) (`self.Atk1PossibleTargets`)
    (if (== _array_element OtherActor)
      (`KismetArrayLibrary.Array_Remove` (`self.Atk1PossibleTargets`) _array_index))))

(fn `ApplyLaunch`
  (params (TargetChar :type "Character Object Reference") (MyChar :type "Actor Object Reference"))
  (locals (NewLocalVar_0 :type "Float (double-precision)" :default 0.0))
  (bind _charactermovement (`Character.CharacterMovement` TargetChar))
  (set `self.OldFriction` (`CharacterMovementComponent.GroundFriction` _charactermovement))
  (set `CharacterMovementComponent.GroundFriction` 0.0 _charactermovement)
  (`CharacterMovementComponent.AddImpulse` (`Character.CharacterMovement` TargetChar) (90000.0 0.0 9000.0) true))

(fn `GetCharToATK`
  (returns (CharATKed :type "/Game/TED_Specific/Character_Assets/Personagem_Generico_BP Object Reference"))
  (bind _asplayer_controller_bp (cast `/Game/TED_Specific/Character_Assets/Player_Controller_BP` (`GameplayStatics.GetPlayerController` 0)))
  (bind _targetchar (`/Game/TED_Specific/Character_Assets/Player_Controller_BP.TargetChar` _asplayer_controller_bp))
  (if (`PrimitiveComponent.IsOverlappingActor` (`self.Atk1_Collider`) _targetchar)
    (`KismetSystemLibrary.PrintString` "achei")
    (set `self.CharToAtk` _targetchar)
    (else
      (set `self.CharToAtk` (`self.NewVar_0`))))
  (return _targetchar))

(fn `UserConstructionScript`
  (`parent.UserConstructionScript`)
  (set `self.CurHealth` 100)
  (set `self.InitHealth` 100)
  (set `self.MaxHealth` 100))